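; Civilian NPC that roams at random and shows a random line of dialogue when interacted with.
; RandomRoam moves to reachable points within RoamingRadius, re-calling itself after each successful move.
; A box overlap with the player shows an interact prompt; leaving clears both widgets and restarts roaming.
; InteractwithCivilillian uses a FlipFlop to alternate between dialogue with a destination-less AIMoveTo and roaming with the prompt, regardless of overlap state.
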(event OnComponentBeginOverlap(Box)
  (params (OverlappedComponent :type Primitive%20Component%20Object%20Reference) (OtherActor :type Actor%20Object%20Reference) (OtherComp :type Primitive%20Component%20Object%20Reference) (OtherBodyIndex :type Integer) (bFromSweep :type Boolean) (SweepResult :type Hit%20Result%20Structure%20%28by%20ref%29))
  ;[0 0.008249 0.15 0.5] On Overlap
  (Utilities|Casting|CastToBP_ThirdPersonCharacter OtherActor)
  (Variables|Default|Setis%20overlapped%20with%20box? true)
  (UserInterface|Viewport|AddtoViewport (Variables|Default|GetWB_Interact) 0))

(event OnComponentEndOverlap(Box)
  (params (OverlappedComponent :type Primitive%20Component%20Object%20Reference) (OtherActor :type Actor%20Object%20Reference) (OtherComp :type Primitive%20Component%20Object%20Reference) (OtherBodyIndex :type Integer))
  ;[0 0.008249 0.15 0.5] On Overlap
  (Utilities|Casting|CastToBP_ThirdPersonCharacter OtherActor)
  (Variables|Default|Setis%20overlapped%20with%20box? false)
  (Variables|Default|SetDailogue%20shown false)
  (Widget|RemovefromParent (Variables|Default|GetWB_Interact))
  (CallFunction|RandomRoam)
  (Widget|RemovefromParent (Variables|Default|GetWB_Dailogue)))

(event Custom|RandomRoam
  ;[0 0.01831 0.15 0.5] Begin Play
  (if (not (Variables|Default|GethasInteracted>))
    (AI|AIMoveTo self (.RandomLocation (AI|Navigation|GetRandomReachablePointinRadius (Transformation|GetActorLocation) (Variables|Default|Getroaming%20Radius) 0 0)) 0 5.0 false
      (:OnSuccess
        (Utilities|FlowControl|Delay 0.2)
        (CallFunction|RandomRoam)))))

(event EventBeginPlay
  (CallFunction|RandomRoam)
  (bind _returnvalue (UserInterface|CreateWidget "/Game/AI/Civilian/Dailogue.Dailogue_C"))
  (Variables|Default|SetWB_Dailogue _returnvalue)
  (bind _returnvalue_2 (UserInterface|CreateWidget "/Game/AI/Quest_AI/Interact.Interact_C"))
  (Variables|Default|SetWB_Interact _returnvalue_2))

(event Collision|EventActorBeginOverlap
  (params (OtherActor :type Actor%20Object%20Reference)))

(event EventTick
  (params (DeltaSeconds :type Float%20%28single-precision%29)))

(event EventInteractwithCivilillian
  ;[0 0.007824 0.15 0.5] Interaction logic
  (Utilities|FlowControl|FlipFlop
    (:A
      (if (and (Variables|Default|Getis%20overlapped%20with%20box?) (not (Variables|Default|GetDailogue%20shown)))
        _
        (else
          _))
      (Variables|/Script/UMG.TextBlock|SetText (Variables|/Game/AI/Civilian/Dailogue.Dailogue_C|GetDailoguetext (Variables|Default|GetWB_Dailogue)) (Utilities|Text|ToText(String) (Utilities|Array|Get(acopy) (Variables|Default|GetDailogue) (Math|Random|RandomIntegerinRange 0 (Variables|Default|Getdailogue%20index)))))
      (UserInterface|Viewport|AddtoViewport (Variables|Default|GetWB_Dailogue) 0)
      (Variables|Default|SetDailogue%20shown true)
      (Widget|RemovefromParent (Variables|Default|GetWB_Interact))
      (AI|AIMoveTo self "0, 0, 0" 0 5.0 false))
    (:B
      (CallFunction|RandomRoam)
      (UserInterface|Viewport|AddtoViewport (Variables|Default|GetWB_Interact) 0)
      (Widget|RemovefromParent (Variables|Default|GetWB_Dailogue)))))

(fn ConstructionScript)